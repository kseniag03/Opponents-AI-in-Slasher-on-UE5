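; BP_CombatManager is an AI manager that limits how many enemies attack one AttackTarget at the same time.
; On BeginPlay it reads the attacker cap from the target through a message call.
; HandleAttackRequest ignores the target itself, adds attackers to Enemies while slots remain, and puts the rest in WaitingEnemies.
; Each requester is messaged to attack or wait; nothing here frees slots or promotes waiting enemies.
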(event EventBeginPlay
  (bind _count (Class|BPIAttackTarget|GetMaxAttackersCount(Message) (Variables|Default|GetAttackTarget)))
  (Variables|Default|SetMaxAttackersCount _count))

(event Collision|EventActorBeginOverlap
  (params (OtherActor :type Actor%20Object%20Reference)))

(event EventTick
  (params (DeltaSeconds :type Float%20%28single-precision%29)))

(fn ConstructionScript)

(fn HandleAttackRequest
  (params (Attacker :type Actor%20Object%20Reference))
  (bind _attacktarget (Variables|Default|GetAttackTarget))
  (if (!= Attacker (Variables|Default|GetAttackTarget))
    (if (< (Utilities|Array|Length (Variables|Default|GetEnemies)) (Variables|Default|GetMaxAttackersCount))
      (Utilities|Array|AddUnique (Variables|Default|GetEnemies) Attacker)
      (Class|BPIAttacker|AttackTarget(Message) Attacker _attacktarget)
      (else
        (Utilities|Array|AddUnique (Variables|Default|GetWaitingEnemies) Attacker)
        (Class|BPIAttacker|WaitBeforeAttack(Message) Attacker _attacktarget)))))