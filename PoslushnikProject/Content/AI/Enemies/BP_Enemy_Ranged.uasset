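; Ranged enemy AI character that attacks by throwing the vase held in its hand.
; It spawns a vase into its hand socket on BeginPlay, and Attack plays a montage whose notifies drive the throw and respawn.
; The drop notify destroys the held vase and calls BPCAttacks.ThrowItem from its location if the AI controller's target is valid.
; It also defines movement speeds and attack and defend ranges.
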(event EventBeginPlay
  (|CallParentFunction)
  (CallFunction|EquipWeapon))

(event EventUnequipWeapon
  (Actor|DestroyActor (Variables|Default|GetWeaponMesh))
  (Variables|Default|SetHasWeapon false)
  (Default|CallOnWeaponUnequipped))

(event EventAttack
  (bind _notifyname (Animation|Montage|PlayMontage (Variables|Character|GetMesh) "/Game/PrototypeNonEditable/Characters/Mannequins/Animations/SwordSlash_Montage.SwordSlash_Montage")
    (:OnCompleted
      (Default|CallOnAttackEnd :!label _label))
    (:OnInterrupted
      (goto _label))
    (:OnNotifyBegin
      (switch name _notifyname
        (:DropWeapon
          (bind _output_get (Variables|Default|SetDroppedWeaponLocation (Transformation|GetActorLocation (Variables|Default|GetWeaponMesh))))
          (CallFunction|UnequipWeapon)
          (bind _asbp_aicontroller (Utilities|Casting|CastToBP_AIController (AI|GetAIController self)))
          (Variables|/Game/AI/Enemies/BP_AIController.BP_AIController_C|GetAttack%20Target _asbp_aicontroller
            (:then
              (Default|ThrowItem (Variables|Default|GetBPC_Attacks) _output_get (Transformation|GetActorLocation) (Utilities|Struct|MakeS_DamageInfo 15.0 "NewEnumerator2")))
            (:else)))
        (:SpawnWeapon
          (if (not (Variables|Default|GetHasWeapon))
            (bind _returnvalue (Game|SpawnActorfromClass "/Game/AI/Weapons/BP_Weapon_Vase.BP_Weapon_Vase_C" (Transformation|GetActorTransform) "Undefined" "MultiplyWithRoot" 0 0))
            (bind _output_get_2 (Variables|Default|SetWeaponMesh _returnvalue))
            (bind _returnvalue_2 (Transformation|AttachComponentToComponent _output_get_2 (Variables|Character|GetMesh) "hand_r_sword_socket" "SnapToTarget" "SnapToTarget" "SnapToTarget" true))
            (Variables|Default|SetHasWeapon _returnvalue_2)
            (Default|CallOnWeaponEquipped)))))))

(event EventEquipWeapon
  (bind _returnvalue (Game|SpawnActorfromClass "/Game/AI/Weapons/BP_Weapon_Vase.BP_Weapon_Vase_C" (Transformation|GetActorTransform) "Undefined" "MultiplyWithRoot" 0 0))
  (bind _output_get (Variables|Default|SetWeaponMesh _returnvalue))
  (bind _returnvalue_2 (Transformation|AttachComponentToComponent _output_get (Variables|Character|GetMesh) "hand_r_sword_socket" "SnapToTarget" "SnapToTarget" "SnapToTarget" true))
  (Variables|Default|SetHasWeapon _returnvalue_2)
  (Default|CallOnWeaponEquipped))

(fn ConstructionScript
  (|CallParentFunction))

(fn SetMovementSpeed
  (params (SpeedType :type E_MovementSpeed%20Enum :default "NewEnumerator0"))
  (bind _output_get (Variables|/Script/Engine.CharacterMovementComponent|SetMaxWalkSpeed (Variables|Character|GetCharacterMovement) (Utilities|Select :Index SpeedType :NewEnumerator0 5e+02 :NewEnumerator1 0.0 :NewEnumerator2 2e+02 :NewEnumerator3 7.5e+02 :NewEnumerator4 1e+03)))
  (return _output_get))

(fn GetProperRange
  (return 6e+02 6e+02))