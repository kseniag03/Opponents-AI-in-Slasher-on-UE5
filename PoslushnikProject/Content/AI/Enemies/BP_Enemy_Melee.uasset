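; Melee enemy that equips a sword, attacks, blocks and exposes a patrol route.
; Equip spawns and socket-attaches the sword, unequip destroys it, and both fire dispatchers.
; Attack plays a slash montage, sphere-tracing forward on its notify to send damage, with the damage component uninterruptible until the montage ends.
; Blocking flags the damage component and plays a forward-roll montage, with no reset here.
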(event Custom|PlayAttackAnimation
  (bind _returnvalue (Transformation|GetActorLocation))
  (bind _notifyname (Animation|Montage|PlayMontage (Variables|Character|GetMesh) "/Game/PrototypeNonEditable/Characters/Mannequins/Animations/SwordSlash_Montage.SwordSlash_Montage")
    (:then
      (Variables|/Game/DamageSystem/BPC_DamageSystem.BPC_DamageSystem_C|SetIsInterruptible (Variables|Default|GetBPC_DamageSystem) false))
    (:OnCompleted
      (Default|CallOnAttackEnd :!label _label)
      (Variables|/Game/DamageSystem/BPC_DamageSystem.BPC_DamageSystem_C|SetIsInterruptible (Variables|Default|GetBPC_DamageSystem) true))
    (:OnInterrupted
      (goto _label))
    (:OnNotifyBegin
      (switch name _notifyname
        (:DropWeapon
          (bind (_outhit _returnvalue_2) (Collision|SphereTraceForObjects _returnvalue (+ _returnvalue (* (Transformation|GetActorForwardVector) 2e+02)) 2e+01 (Utilities|Array|MakeArray "ObjectTypeQuery3") false 0 "ForDuration"))
          (if _returnvalue_2
            (Class|BPIDamageable|TakeDamage(Message) (.HitActor (Collision|BreakHitResult _outhit)) (Utilities|Struct|MakeS_DamageInfo 15.0 "NewEnumerator1"))))))))

(event Custom|StartBlock
  (Variables|/Game/DamageSystem/BPC_DamageSystem.BPC_DamageSystem_C|SetIsBlocking (Variables|Default|GetBPC_DamageSystem) true)
  (Animation|Montage|PlayMontage (Variables|Character|GetMesh) "/Game/ThirdPerson/Blueprints/Dodge_Small_Forward_Roll_Montage.Dodge_Small_Forward_Roll_Montage"))

(event EventBeginPlay
  (|CallParentFunction) ; This node is disabled and will not be called.\nDrag off pins to build functionality.
)

(event EventEquipWeapon
  (bind _returnvalue (Game|SpawnActorfromClass "/Game/AI/Weapons/BP_Weapon_Sword.BP_Weapon_Sword_C" (Transformation|GetActorTransform) "Undefined" "MultiplyWithRoot" 0 0))
  (bind _output_get (Variables|Default|SetWeaponMesh _returnvalue))
  (Transformation|AttachComponentToComponent _output_get (Variables|Character|GetMesh) "hand_r_sword_socket" "SnapToTarget" "SnapToTarget" "SnapToTarget" true)
  (Variables|Default|SetHasWeapon true)
  (Utilities|FlowControl|Delay 0.2)
  (Default|CallOnWeaponEquipped))

(event EventTick
  (params (DeltaSeconds :type Float%20%28single-precision%29)))

(event EventUnequipWeapon
  (Actor|DestroyActor (Variables|Default|GetWeaponMesh))
  (Variables|Default|SetHasWeapon false)
  (Default|CallOnWeaponUnequipped))

(event Collision|EventActorBeginOverlap
  (params (OtherActor :type Actor%20Object%20Reference)))

(event EventAttack
  (CallFunction|PlayAttackAnimation))

(fn ConstructionScript
  (|CallParentFunction))

(fn GetPatrolRoute
  (return (Variables|Default|GetPatrolRoute)))