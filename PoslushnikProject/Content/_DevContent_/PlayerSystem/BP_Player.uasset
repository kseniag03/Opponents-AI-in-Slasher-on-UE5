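; Player character with sword melee, a fireball spell, and health, mana and stamina handled by components.
; A looping timer traces between sockets on the spawned sword to damage enemies, while a montage notify spawns fireballs.
; Incoming damage passes through the damage system component, triggering hit reaction, noise and particles; death is forwarded to the player controller.
; Wrapper functions expose component stats, and running out of stamina resets walk speed to default.
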(event Custom|StopSprint
  ;[1 1 1] Start settings
  (Development|PrintString "DEFAULT SPEED")
  (CallFunction|SetMovementSpeed "NewEnumerator0"))

(event Custom|DealWithDamage
  (bind _returnvalue (Transformation|GetActorLocation))
  ;[1 1 1] Deal with damage
  (Animation|Montage|PlayMontage (Variables|Character|GetMesh) "/Game/PrototypeNonEditable/Characters/Mannequins/Animations/HitReact_Montage.HitReact_Montage"
    (:then
      (Class|Actor|MakeNoise 1.0 self _returnvalue 1e+02 "None")
      (Effects|SpawnEmitteratLocation "/Game/StarterContent/Particles/P_Explosion.P_Explosion" _returnvalue))))

(event Custom|TriggerWeapon
  ;[1 1 1] Perform player attack
  (bind _returnvalue (Utilities|Time|SetTimerbyEvent (delegate Custom|WeaponLinetrace) 0.01 true))
  (Variables|Default|SetTriggerWeaponEvent _returnvalue))

(event Custom|PlayerDeath
  ;[1 1 1] Implement death ising Observer & Component pattern
  (bind _asbp_player_controller (Utilities|Casting|CastToBP_PlayerController (Game|GetPlayerController 0)))
  (Default|Death _asbp_player_controller))

(event Custom|SpellCast
  ;[1 1 1] Perform Projectile Player Attack
  (Utilities|FlowControl|DoOnce false :!label _label
    (:Completed
      (bind _notifyname (Animation|Montage|PlayMontage (Variables|Character|GetMesh) "/Game/_DevContent_/Montage/M_FireballCast.M_FireballCast")
        (:OnCompleted
          (goto _label Reset))
        (:OnNotifyBegin
          (switch name _notifyname
            (:Cast
              (Game|SpawnActorfromClass "/Game/_DevContent_/Components/DamageSystem/Attacks/Spell/BP_Fireball.BP_Fireball_C" (Transformation|GetWorldTransform (Variables|Default|GetCastDirection)) "Undefined" "MultiplyWithRoot" 0 0))))))))

(event Custom|EndTriggerWeapon
  ;[1 1 1] Perform player attack
  (Utilities|Time|ClearandInvalidateTimerbyHandle (Variables|Default|GetTriggerWeaponEvent)))

(event Custom|WeaponLinetrace
  ;[1 1 1] Perform player attack
  (|PlayerMeleeTraces))

(event Game|Damage|EventAnyDamage
  (params (Damage :type Float%20%28single-precision%29) (DamageType :type Damage%20Type%20Object%20Reference) (InstigatedBy :type Controller%20Object%20Reference) (DamageCauser :type Actor%20Object%20Reference))
  ;[1 1 1] Process environment damage
  (CallFunction|TakeDamage (Utilities|Struct|MakeS_DamageInfo Damage "NewEnumerator4")))

(event EventBeginPlay
  ;[1 1 1] Start settings
  (|SpawnPlayerSword)
  (bind _returnvalue (Actor|GetActorOfClass "/Game/_DevContent_/AISystem/Managers/BP_CombatManager.BP_CombatManager_C"))
  (Variables|Default|SetCombatManager _returnvalue)
  (EventDispatchers|BindEventtoOnAllStaminaSpent (Variables|Default|GetBP_StaminaComp) (delegate Custom|StopSprint)))

(fn ConstructionScript
  (EventDispatchers|BindEventtoOnDeath (Variables|Default|GetBPC_DamageSystem) (EventDispatchers|CreateEvent :!event Custom|PlayerDeath)))

(fn CanCast
  (params (SpellCost :type Float%20%28double-precision%29))
  (bind _cancast (Default|CanCast (Variables|Default|GetBP_ManaComp) SpellCost))
  (return _cancast))

(fn FillMana
  (params (Amount :type Float%20%28double-precision%29))
  (bind _curmana (Default|FillMana (Variables|Default|GetBP_ManaComp) Amount))
  (return _curmana))

(fn FillStamina
  (params (Amount :type Float%20%28double-precision%29))
  (bind _curstamina (Default|FillStamina (Variables|Default|GetBP_StaminaComp) Amount))
  (return _curstamina))

(fn GetCurHealth
  (return (Variables|/Game/_DevContent_/Components/BPC_HealthComp.BPC_HealthComp_C|GetCurHealth (Variables|Default|GetBP_HealthComp))))

(fn GetCurMana
  (return (Variables|/Game/_DevContent_/Components/BPC_ManaComp.BPC_ManaComp_C|GetCurMana (Variables|Default|GetBP_ManaComp))))

(fn GetCurStamina
  (return (Variables|/Game/_DevContent_/Components/BPC_StaminaComp.BPC_StaminaComp_C|GetCurStamina (Variables|Default|GetBP_StaminaComp))))

(fn GetMaxAttackersCount
  (bind _asbp_game_mode (Utilities|Casting|CastToBP_GameMode (Game|GetGameMode)))
  (return (Variables|/Game/_DevContent_/GameSystem/BP_GameMode.BP_GameMode_C|GetMaxPlayerAttackersCount _asbp_game_mode)))

(fn GetMaxHealth
  (return (Variables|/Game/_DevContent_/Components/BPC_HealthComp.BPC_HealthComp_C|GetMaxHealth (Variables|Default|GetBP_HealthComp))))

(fn GetMaxMana
  (return (Variables|/Game/_DevContent_/Components/BPC_ManaComp.BPC_ManaComp_C|GetMaxMana (Variables|Default|GetBP_ManaComp))))

(fn GetMaxStamina
  (return (Variables|/Game/_DevContent_/Components/BPC_StaminaComp.BPC_StaminaComp_C|GetMaxStamina (Variables|Default|GetBP_StaminaComp))))

(fn GetName
  (return "Player"))

(fn Heal
  (params (Amount :type Float%20%28double-precision%29))
  (return 0.0))

(fn IsDead
  (return (Variables|/Game/_DevContent_/Components/BPC_HealthComp.BPC_HealthComp_C|GetIsDead (Variables|Default|GetBP_HealthComp))))

(fn IsManaNotFull
  (bind _bp_manacomp (Variables|Default|GetBP_ManaComp))
  (return (and (Variables|/Game/_DevContent_/Components/BPC_ManaComp.BPC_ManaComp_C|GetCanFill _bp_manacomp) (Variables|/Game/_DevContent_/Components/BPC_ManaComp.BPC_ManaComp_C|GetIsPraying _bp_manacomp))))

(fn IsStaminaNotEmpty
  (return (Variables|/Game/_DevContent_/Components/BPC_StaminaComp.BPC_StaminaComp_C|GetCanRun (Variables|Default|GetBP_StaminaComp))))

(fn IsStaminaNotFull
  (return (Variables|/Game/_DevContent_/Components/BPC_StaminaComp.BPC_StaminaComp_C|GetCanFill (Variables|Default|GetBP_StaminaComp))))

(fn SetMovementSpeed
  (params (SpeedType :type E_MovementSpeed%20Enum :default "NewEnumerator0"))
  (bind _output_get (Variables|/Script/Engine.CharacterMovementComponent|SetMaxWalkSpeed (Variables|Character|GetCharacterMovement) (Utilities|Select :Index SpeedType :NewEnumerator0 5e+02 :NewEnumerator1 0.0 :NewEnumerator2 1e+02 :NewEnumerator3 7.5e+02 :NewEnumerator4 1e+03)))
  (return _output_get))

(fn SetupCanFill
  (params (NewCanFill :type Boolean))
  (bind _output_get (Variables|/Game/_DevContent_/Components/BPC_StaminaComp.BPC_StaminaComp_C|SetCanFill (Variables|Default|GetBP_StaminaComp) NewCanFill))
  (return _output_get))

(fn SetupCanRun
  (params (NewCanRun :type Boolean))
  (bind _output_get (Variables|/Game/_DevContent_/Components/BPC_StaminaComp.BPC_StaminaComp_C|SetCanRun (Variables|Default|GetBP_StaminaComp) NewCanRun))
  (return _output_get))

(fn TakeDamage
  (params (DamageInfo :type S%20Damage%20Info%20Structure))
  (bind _wasdamaged (Default|TakeDamage (Variables|Default|GetBPC_DamageSystem) DamageInfo (Variables|Default|GetBP_HealthComp)))
  (if _wasdamaged
    (CallFunction|DealwithDamage)
    (return _wasdamaged)))

(fn WasteMana
  (params (Amount :type Float%20%28double-precision%29))
  (bind _curmana (Default|WasteMana (Variables|Default|GetBP_ManaComp) Amount))
  (return _curmana))

(fn WasteStamina
  (params (Amount :type Float%20%28double-precision%29))
  (bind _curstamina (Default|WasteStamina (Variables|Default|GetBP_StaminaComp) Amount))
  (return _curstamina))