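; BP_Teleport is a level trigger that sends the player to the next lobby when they cross a door.
; Its box overlap checks for player character 0, then teleports it to the next lobby location from BP_GameInstance with zero rotation.
; It then calls its own OnPlayerTeleport and notifies BP_GameState through OnPlayerTeleported.
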(event OnComponentBeginOverlap(Box)
  (params (OverlappedComponent :type Primitive%20Component%20Object%20Reference) (OtherActor :type Actor%20Object%20Reference) (OtherComp :type Primitive%20Component%20Object%20Reference) (OtherBodyIndex :type Integer) (bFromSweep :type Boolean) (SweepResult :type Hit%20Result%20Structure%20%28by%20ref%29))
  ;[1 1 1] Teleport the player crossing the door to the next lobby
  (if (== OtherActor (Game|GetPlayerCharacter 0))
    (bind _asbp_game_instance (Utilities|Casting|CastToBP_GameInstance (Game|GetGameInstance)))
    (bind _location (Default|GetNextLobbyLocation _asbp_game_instance))
    (Transformation|Teleport OtherActor _location "0, 0, 0")
    (Default|CallOnPlayerTeleport)
    (bind _asbp_game_state (Utilities|Casting|CastToBP_GameState (Game|GetGameState)))
    (Default|CallOnPlayerTeleported _asbp_game_state)))

(fn ConstructionScript)