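; BP_CombatManager limits how many enemies attack one target at once, defaulting to the player character, whose message sets the attacker cap.
; Attack requests fill an active list up to the cap, with overflow queued as waiting.
; An active attacker's death promotes the first waiting enemy, while the target's death sends all enemies to patrol.
; Both lists clear when the game state reports a player teleport.
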(event Custom|ClearEnemies
  (Utilities|Array|Clear (Variables|Default|GetActiveEnemies))
  (Utilities|Array|Clear (Variables|Default|GetWaitingEnemies)))

(event EventBeginPlay
  (bind _attacktarget (Variables|Default|GetAttackTarget)
    (:then
      _)
    (:else
      (Variables|Default|SetAttackTarget (Game|GetPlayerCharacter 0))))
  (bind _count (Class|BPIAttackTarget|GetMaxAttackersCount(Message) _attacktarget))
  (Variables|Default|SetMaxAttackersCount _count)
  (bind _asbp_game_state (Utilities|Casting|CastToBP_GameState (Game|GetGameState)))
  (EventDispatchers|BindEventtoOnPlayerTeleported _asbp_game_state (delegate Custom|ClearEnemies)))

(fn ConstructionScript)

(fn HandleAttackRequest
  (params (Attacker :type Actor%20Object%20Reference))
  (if (!= Attacker (Variables|Default|GetAttackTarget))
    (if (< (Utilities|Array|Length (Variables|Default|GetActiveEnemies)) (Variables|Default|GetMaxAttackersCount))
      (Utilities|Array|AddUnique (Variables|Default|GetActiveEnemies) Attacker)
      (else
        (Utilities|Array|AddUnique (Variables|Default|GetWaitingEnemies) Attacker)))))

(fn HandleDeath
  (params (Actor :type Actor%20Object%20Reference))
  (bind _activeenemies (Variables|Default|GetActiveEnemies))
  (bind _output_get (Variables|Default|SetDeadActor Actor))
  (if (== _output_get (Variables|Default|GetAttackTarget))
    (Utilities|Array|AppendArray _activeenemies (Variables|Default|GetWaitingEnemies))
    (for _array_element _activeenemies
      (Class|BPIAttacker|PatrolasTargetIsDead(Message) _array_element))
    (Utilities|Array|Clear (Variables|Default|GetActiveEnemies))
    (Utilities|Array|Clear (Variables|Default|GetWaitingEnemies))
    (elif (Utilities|Array|ContainsItem (Variables|Default|GetActiveEnemies) (Variables|Default|GetDeadActor))
      (Utilities|Array|RemoveItem (Variables|Default|GetActiveEnemies) (Variables|Default|GetDeadActor))
      (CallFunction|MoveWaitingEnemies)
      (elif (Utilities|Array|ContainsItem (Variables|Default|GetWaitingEnemies) (Variables|Default|GetDeadActor))
        (Utilities|Array|RemoveItem (Variables|Default|GetWaitingEnemies) (Variables|Default|GetDeadActor))))))

(fn MoveWaitingEnemies
  (bind _waitingenemies (Variables|Default|GetWaitingEnemies))
  (bind _output (Utilities|Array|Get(acopy) _waitingenemies))
  (Utilities|IsValid _output
    (:Is%20Valid
      (bind _output_get (Variables|Default|SetCurWaitingEnemy _output))
      (Utilities|Array|RemoveItem (Variables|Default|GetWaitingEnemies) _output_get)
      (Utilities|Array|AddUnique (Variables|Default|GetActiveEnemies) (Variables|Default|GetCurWaitingEnemy)))))

(fn IsActiveAttacker
  (params (Attacker :type Actor%20Object%20Reference))
  (return (Utilities|Array|ContainsItem (Variables|Default|GetActiveEnemies) Attacker)))

(fn IsWaitingAttacker
  (params (Attacker :type Actor%20Object%20Reference))
  (return (Utilities|Array|ContainsItem (Variables|Default|GetWaitingEnemies) Attacker)))