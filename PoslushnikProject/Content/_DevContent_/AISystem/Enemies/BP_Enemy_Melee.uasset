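; Melee AI enemy named "Duelist" that fights with a sword and supplies its patrol route, combat ranges and movement speeds.
; It spawns and attaches the sword to a hand socket, then signals equip completion.
; Blocking sets a damage-system flag and plays a roll montage.
; Attacks play a slash montage whose notify triggers a forward sphere trace, dealing GameMode-defined damage to the pawn hit, and signal attack end on completion or interruption.
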(event Custom|StartBlock
  (Variables|/Game/_DevContent_/Components/DamageSystem/BPC_DamageSystem.BPC_DamageSystem_C|SetIsBlocking (Variables|Default|GetBPC_DamageSystem) true)
  (Animation|Montage|PlayMontage (Variables|Character|GetMesh) "/Game/ThirdPerson/Blueprints/Dodge_Small_Forward_Roll_Montage.Dodge_Small_Forward_Roll_Montage"))

(event EventBeginPlay
  (|CallParentFunction) ; This node is disabled and will not be called.\nDrag off pins to build functionality.
)

(event EventEquipWeapon
  ;[1 1 1] Equip weapon (sword)
  (bind _returnvalue (Game|SpawnActorfromClass "/Game/_DevContent_/Components/DamageSystem/Attacks/Weapons/BP_Weapon_Sword.BP_Weapon_Sword_C" (Transformation|GetActorTransform) "Undefined" "MultiplyWithRoot" 0 0))
  (bind _output_get (Variables|Default|SetWeaponMesh _returnvalue))
  (bind _returnvalue_2 (Transformation|AttachComponentToComponent _output_get (Variables|Character|GetMesh) "hand_r_sword_socket" "SnapToTarget" "SnapToTarget" "SnapToTarget" true))
  (Variables|Default|SetHasWeapon _returnvalue_2)
  (Utilities|FlowControl|Delay 0.2)
  (Default|CallOnWeaponEquipped))

(event EventAttackTarget
  (params (AttackTarget :type Actor%20Object%20Reference))
  (bind _returnvalue (Transformation|GetActorLocation))
  ;[1 1 1] Perform melee attack
  (bind _notifyname (Animation|Montage|PlayMontage (Variables|Character|GetMesh) "/Game/_DevContent_/Montage/M_SwordSlash.M_SwordSlash")
    (:then
      (Variables|/Game/_DevContent_/Components/DamageSystem/BPC_DamageSystem.BPC_DamageSystem_C|SetIsInterruptible (Variables|Default|GetBPC_DamageSystem) false :!label _label))
    (:OnCompleted
      (Default|CallOnAttackEnd :!label _label_2)
      (goto _label))
    (:OnInterrupted
      (goto _label_2))
    (:OnNotifyBegin
      (switch name _notifyname
        (:DropWeapon
          (bind (_outhit _returnvalue_2) (Collision|SphereTraceForObjects _returnvalue (+ _returnvalue (* (Transformation|GetActorForwardVector) 2e+02)) 2e+01 (Utilities|Array|MakeArray "ObjectTypeQuery3") false 0 "ForDuration"))
          (if _returnvalue_2
            (bind _asbp_game_mode (Utilities|Casting|CastToBP_GameMode (Game|GetGameMode)))
            (Class|BPIDamagable|TakeDamage(Message) (.HitActor (Collision|BreakHitResult _outhit)) (Utilities|Struct|MakeS_DamageInfo (Variables|/Game/_DevContent_/GameSystem/BP_GameMode.BP_GameMode_C|GetBaseMeleeEnemyDamage _asbp_game_mode) "NewEnumerator1"))))))))

(fn ConstructionScript
  (|CallParentFunction))

(fn GetPatrolRoute
  (return (Variables|Default|GetPatrolRoute)))

(fn GetProperRange
  (return 1e+02 2e+02))

(fn SetMovementSpeed
  (params (SpeedType :type E_MovementSpeed%20Enum :default "NewEnumerator0"))
  (bind _output_get (Variables|/Script/Engine.CharacterMovementComponent|SetMaxWalkSpeed (Variables|Character|GetCharacterMovement) (Utilities|Select :Index SpeedType :NewEnumerator0 4e+02 :NewEnumerator1 0.0 :NewEnumerator2 1e+02 :NewEnumerator3 5.5e+02 :NewEnumerator4 7.5e+02)))
  (return _output_get))

(fn GetName
  (return "Duelist"))