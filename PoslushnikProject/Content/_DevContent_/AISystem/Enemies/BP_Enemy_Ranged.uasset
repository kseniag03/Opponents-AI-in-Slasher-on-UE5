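; BP_Enemy_Ranged is the "Thrower" enemy, which spawns a vase weapon into its hand on BeginPlay and throws it as a ranged attack.
; The attack montage's notifies drive the cycle: one unequips the vase and calls BPCAttacks.ThrowItem with game-mode damage if the AI controller's target is valid, another re-equips.
; It also supplies its own movement speeds, attack and defend radii, and name.
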(event EventBeginPlay
  (|CallParentFunction)
  (CallFunction|EquipWeapon))

(event EventAttackTarget
  (params (AttackTarget :type Actor%20Object%20Reference))
  ;[1 1 1] Perform projectile attack
  (bind _notifyname (Animation|Montage|PlayMontage (Variables|Character|GetMesh) "/Game/_DevContent_/Montage/M_SwordSlash.M_SwordSlash")
    (:OnCompleted
      (Default|CallOnAttackEnd :!label _label))
    (:OnInterrupted
      (goto _label))
    (:OnNotifyBegin
      (switch name _notifyname
        (:DropWeapon
          (Variables|Default|SetDroppedWeaponLocation (Transformation|GetActorLocation (Variables|Default|GetWeaponMesh)))
          (CallFunction|UnequipWeapon)
          (bind _asbp_aicontroller (Utilities|Casting|CastToBP_AIController (AI|GetAIController self)))
          (Variables|/Game/_DevContent_/AISystem/Enemies/BP_AIController.BP_AIController_C|GetAttack%20Target _asbp_aicontroller
            (:then
              (bind _asbp_game_mode (Utilities|Casting|CastToBP_GameMode (Game|GetGameMode)))
              (Default|ThrowItem (Variables|Default|GetBPC_Attacks) "0, 0, 0" (Transformation|GetActorLocation) (Utilities|Struct|MakeS_DamageInfo (Variables|/Game/_DevContent_/GameSystem/BP_GameMode.BP_GameMode_C|GetBaseRangedEnemyDamage _asbp_game_mode) "NewEnumerator2")))
            (:else)))
        (:SpawnWeapon
          (if (not (Variables|Default|GetHasWeapon))
            (CallFunction|EquipWeapon)))))))

(event EventEquipWeapon
  ;[1 1 1] Equip weapon (vase)
  (bind _returnvalue (Game|SpawnActorfromClass "/Game/_DevContent_/Components/DamageSystem/Attacks/Weapons/BP_Weapon_Vase.BP_Weapon_Vase_C" (Transformation|GetActorTransform) "Undefined" "MultiplyWithRoot" 0 0))
  (bind _output_get (Variables|Default|SetWeaponMesh _returnvalue))
  (bind _returnvalue_2 (Transformation|AttachComponentToComponent _output_get (Variables|Character|GetMesh) "hand_r_sword_socket" "SnapToTarget" "SnapToTarget" "SnapToTarget" true))
  (Variables|Default|SetHasWeapon _returnvalue_2)
  (Default|CallOnWeaponEquipped))

(fn ConstructionScript
  (|CallParentFunction))

(fn SetMovementSpeed
  (params (SpeedType :type E_MovementSpeed%20Enum :default "NewEnumerator0"))
  (bind _output_get (Variables|/Script/Engine.CharacterMovementComponent|SetMaxWalkSpeed (Variables|Character|GetCharacterMovement) (Utilities|Select :Index SpeedType :NewEnumerator0 5e+02 :NewEnumerator1 0.0 :NewEnumerator2 2e+02 :NewEnumerator3 7.5e+02 :NewEnumerator4 1e+03)))
  (return _output_get))

(fn GetProperRange
  (return 2e+02 3e+02))

(fn GetName
  (return "Thrower"))