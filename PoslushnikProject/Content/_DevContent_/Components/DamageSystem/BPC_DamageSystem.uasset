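; Damage system component that applies damage and healing to a health component passed into each call.
; TakeDamage uses a CanBeDamaged macro to check death, invincibility and blocking, with per-hit overrides from DamageInfo.
; It clamps health, returns whether damage landed, and fires dispatchers for block (with parry flag), death or interrupting damage response.
; Heal restores a fraction of max health while the target is alive.
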(event EventBeginPlay)

(event EventTick
  (params (DeltaSeconds :type Float%20%28single-precision%29)))

(fn TakeDamage
  (params (DamageInfo :type S%20Damage%20Info%20Structure) (HealthComp :type BPC%20Health%20Comp%20Object%20Reference))
  (bind (_amount _damagetype _damageresponse _shoulddamageinvincible _canbeblocked _canbeparried _shouldforceinterrupt) (Utilities|Struct|BreakS_DamageInfo DamageInfo))
  (bind _output_get (LocalVariables|SetHealthComponent HealthComp))
  (Utilities|CanbeDamaged _shoulddamageinvincible _canbeblocked _output_get
    (:BlockDamage
      (Default|CallOnBlocked _canbeparried))
    (:DoDamage
      (bind _output_get_2 (Variables|/Game/_DevContent_/Components/BPC_HealthComp.BPC_HealthComp_C|SetCurHealth (LocalVariables|GetHealthComponent) (Math|Float|Clamp(Float) (- (Variables|/Game/_DevContent_/Components/BPC_HealthComp.BPC_HealthComp_C|GetCurHealth (LocalVariables|GetHealthComponent)) _amount) 0.0 (Variables|/Game/_DevContent_/Components/BPC_HealthComp.BPC_HealthComp_C|GetMaxHealth (LocalVariables|GetHealthComponent)))))
      (if (<= _output_get_2 0.0)
        (Variables|/Game/_DevContent_/Components/BPC_HealthComp.BPC_HealthComp_C|SetIsDead (LocalVariables|GetHealthComponent) true)
        (Default|CallOnDeath)
        (elif (or (Variables|Default|GetIsInterruptible) _shouldforceinterrupt)
          (Default|CallOnDamageResponse)))
      (return true))
    (:NoDamage
      _))
  (return false))

(fn Heal
  (params (Amount :type Float%20%28double-precision%29) (HealthComp :type BPC%20Health%20Comp%20Object%20Reference))
  (bind _output_get (LocalVariables|SetHealthComponent HealthComp))
  (if (not (Variables|/Game/_DevContent_/Components/BPC_HealthComp.BPC_HealthComp_C|GetIsDead _output_get))
    (bind _output_get_2 (Variables|/Game/_DevContent_/Components/BPC_HealthComp.BPC_HealthComp_C|SetCurHealth (LocalVariables|GetHealthComponent) (Math|Float|Clamp(Float) (+ (Variables|/Game/_DevContent_/Components/BPC_HealthComp.BPC_HealthComp_C|GetCurHealth (LocalVariables|GetHealthComponent)) (* Amount (Variables|/Game/_DevContent_/Components/BPC_HealthComp.BPC_HealthComp_C|GetMaxHealth (LocalVariables|GetHealthComponent)))) 0.0 (Variables|/Game/_DevContent_/Components/BPC_HealthComp.BPC_HealthComp_C|GetMaxHealth (LocalVariables|GetHealthComponent)))))
    (return _output_get_2)))