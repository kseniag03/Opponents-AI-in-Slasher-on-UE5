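; BP_HealthComp is a health component that stores its owner and tracks current health, maximum health and a dead flag.
; BeginPlay fills health to maximum, and Heal adds points capped at that maximum.
; TakeDamage subtracts clamped damage while alive, prints health and calls Death at zero, which only sets IsDead.
; The binding of TakeDamage to OnTakeAnyDamage is never executed, so this graph does not hook up incoming damage.
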(event Custom|Death
  ;[1 1 1] Old logic
  (Variables|Default|SetIsDead true))

(event Custom|TakeDamage
  (params (DamagedActor :type Actor%20Object%20Reference) (Damage :type Float%20%28single-precision%29) (DamageType :type Damage%20Type%20Object%20Reference) (InstigatedBy :type Controller%20Object%20Reference) (DamageCauser :type Actor%20Object%20Reference))
  ;[1 1 1] Old logic
  (if (not (Variables|Default|GetIsDead))
    (bind _output_get (Variables|Default|SetCurHealth (Math|Float|Clamp(Float) (- (Variables|Default|GetCurHealth) Damage) 0.0 (Variables|Default|GetMaxHealth))))
    (Development|PrintString (Utilities|String|ToString(Float) (Math|Float|Clamp(Float) (- (Variables|Default|GetCurHealth) Damage) 0.0 (Variables|Default|GetMaxHealth))))
    (if (== _output_get 0.0)
      (CallFunction|Death))))

(event Custom|Heal
  (params (HealPoints :type Integer))
  (Variables|Default|SetCurHealth (Math|Float|Min(Float) (Variables|Default|GetMaxHealth) (+ HealPoints (Variables|Default|GetCurHealth)))))

(event EventBeginPlay
  (Variables|Default|SetOwner (Components|GetOwner))
  (bind _output_get (Variables|Default|SetMaxHealth 1e+02))
  (Variables|Default|SetCurHealth _output_get))

(event EventTick
  (params (DeltaSeconds :type Float%20%28single-precision%29)))