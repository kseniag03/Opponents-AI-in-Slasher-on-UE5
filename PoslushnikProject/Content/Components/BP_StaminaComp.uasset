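; BP_StaminaComp is a stamina component that initializes to a full pool on BeginPlay and stores a reference to its owner.
; WasteStamina drains a fixed step per call, clearing IsRunning at zero and otherwise printing the current value.
; FillStamina restores the same step only while not running and sets CanFill until the pool is full.
; Tick is unused, and nothing here schedules either stamina event.
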(event Custom|FillStamina
  (if (not (Variables|Default|GetisRunning))
    (bind _output_get (Variables|Default|SetCurStamina (Math|Float|Clamp(Float) (+ (Variables|Default|GetCurStamina) 5.0) 0.0 (Variables|Default|GetMaxStamina))))
    (if (== _output_get (Variables|Default|GetMaxStamina))
      (Variables|Default|SetcanFill false)
      (else
        (Variables|Default|SetcanFill true)))))

(event Custom|WasteStamina
  (bind _output_get (Variables|Default|SetCurStamina (Math|Float|Clamp(Float) (- (Variables|Default|GetCurStamina) 5.0) 0.0 (Variables|Default|GetMaxStamina))))
  (if (== _output_get 0.0)
    (Variables|Default|SetisRunning false)
    (else
      (Development|PrintString (Utilities|String|ToString(Float) _output_get)))))

(event EventBeginPlay
  (Variables|Default|SetOwner (Components|GetOwner))
  (bind _output_get (Variables|Default|SetMaxStamina 1e+02))
  (Variables|Default|SetCurStamina _output_get))

(event EventTick
  (params (DeltaSeconds :type Float%20%28single-precision%29)))