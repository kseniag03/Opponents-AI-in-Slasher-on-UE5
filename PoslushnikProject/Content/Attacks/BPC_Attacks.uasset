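; BPC_Attacks is a component that gives its owner three attack events: melee, throw and magic spell.
; ThrowItem line-traces for Pawns, sends the hit actor a damage interface message and reports a damage event to AI perception.
; MagicSpell spawns a base Actor at the given transform with the owner set, leaving its damage info unused.
; MeleeAttack is an empty stub.
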(event Custom|MagicSpell
  (params (SpawnTransform :type Transform) (DamageInfo :type S%20Damage%20Info%20Structure))
  (Game|SpawnActorfromClass "/Script/Engine.Actor" SpawnTransform "Undefined" "MultiplyWithRoot" (Components|GetOwner) 0))

(event Custom|ThrowItem
  (params (TraceStart :type Vector) (TraceEnd :type Vector) (DamageInfo :type S%20Damage%20Info%20Structure))
  (bind _returnvalue (Components|GetOwner))
  (bind (_outhit _returnvalue_2) (Collision|LineTraceForObjects TraceStart TraceEnd (Utilities|Array|MakeArray "ObjectTypeQuery3") false 0 "None"))
  (if _returnvalue_2
    (Class|BPIDamagable|TakeDamage(Message) (.HitActor (Collision|BreakHitResult _outhit)) DamageInfo)
    (Class|AISenseDamage|ReportDamageEvent (.HitActor (Collision|BreakHitResult _outhit)) _returnvalue (.Amount (Utilities|Struct|BreakS_DamageInfo DamageInfo)) (Transformation|GetActorLocation _returnvalue) "0, 0, 0" "None")))

(event Custom|MeleeAttack)